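; Game mode for a turn-based multiplayer labyrinth game pitting explorers against one Mummy.
; It triggers labyrinth generation, registers travelled-in controllers, then runs a delayed start sequence syncing collisions, shuffled treasure tiles and explorer invisibility to the Mummy.
; Controller delegates drive turns through each explorer, then the Mummy, with special Mummy turns stepping the index back.
; Explorers win with no treasure tiles left; the Mummy by reaching a lives threshold scaled to explorer count.
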(event Custom|AttemptStartGame
  (if (and (== (Variables|Default|GetNumTravellingPlayers) 0) (not (Variables|Turns|GetHasGameStarted)))
    (Variables|Turns|SetHasGameStarted true)
    (Variables|WinConditions|SetConnectedExplorersAmount (Utilities|Array|Length (Variables|Default|GetConnectedExplorers)))
    (Development|PrintString "Start first player" true true "(R=0.000000,G=0.660000,B=1.000000,A=1.000000)" 5.0)
    (Utilities|FlowControl|Delay 5.0)
    (CallFunction|UpdateClientCollisions)
    (Utilities|FlowControl|Delay 5.0)
    (CallFunction|DistributeTreasureTiles)
    (Development|PrintString "Treasure tiles updated")
    (Utilities|FlowControl|Delay 2.0)
    (CallFunction|PostInitializeControllers)
    (CallFunction|SetExplorersInvisibletoMummy)
    (Development|PrintString "client updated")
    (Utilities|FlowControl|Delay 2.0)
    (CallFunction|OnPlayerTurn)))

(event Custom|FinishPlayerTurn
  (params (IsSpecialTurn :type Boolean))
  (Variables|Turns|SetIs%20Special%20Turn IsSpecialTurn)
  (Variables|Turns|SetDieValues (Variables|/Game/Blueprints/Characters/Player/BP_PlayerController.BP_PlayerController_C|GetDieValues (Variables|Turns|GetCurrentPlayer)))
  (EventDispatchers|UnbindEventfromOnTurnFinished (Variables|Turns|GetCurrentPlayer) (EventDispatchers|CreateEvent :!event Custom|FinishPlayerTurn))
  (EventDispatchers|UnbindEventfromOnTreasureGrabbed (Variables|Turns|GetCurrentPlayer) (EventDispatchers|CreateEvent :!event NotifyTreasureGrabbed))
  (EventDispatchers|UnbindEventfromOnExplorerCaught (Variables|Turns|GetCurrentPlayer) (EventDispatchers|CreateEvent :!event NotifyExplorerCaught))
  (if (CallFunction|HasPlayerWon)
    (Development|PrintString "Player Won!")
    (else
      (Utilities|Time|SetTimerbyEvent (delegate Custom|InitiateNextPlayerTurn) 2.0))))

(event Custom|InitiateNextPlayerTurn
  (Development|PrintString "Next Player Turn" true true "(R=0.000000,G=0.660000,B=1.000000,A=1.000000)" 5.0)
  (CallFunction|OnPlayerTurn))

(event EventOnInitializeGame
  (bind _returnvalue (Actor|GetActorOfClass "/Game/Blueprints/Labyrinth/BP_LabyrinthGenerator.BP_LabyrinthGenerator_C"))
  (Utilities|IsValid _returnvalue
    (:Is%20Valid
      (Class|LabyrinthGenerator|Generate _returnvalue))))

(event EventOnLogout
  (params (ExitingController :type Controller%20Object%20Reference))
  (CallFunction|DisconnectPlayer ExitingController))

(event EventOnSwapPlayerControllers
  (params (OldPC :type Player%20Controller%20Object%20Reference) (NewPC :type Player%20Controller%20Object%20Reference))
  (CallFunction|ConnectPlayer NewPC))

(fn ConstructionScript)

(fn SetLabyrinthTiles
  (params (Tiles :type Array%20of%20Tile%20Base%20Object%20References) (TreasureZones :type Array%20of%20Treasure%20Zone%20Structures))
  (Variables|Labyrinth|SetTiles Tiles)
  (Variables|Labyrinth|SetTreasure%20Zones TreasureZones)
  (Variables|Labyrinth|SetIsLabyrinthReady true))

(fn ChoosePlayerStart
  (params (Player :type Controller%20Object%20Reference))
  (bind _asbp_player_controller (Utilities|Casting|CastToBP_PlayerController Player))
  (Development|PrintString (Utilities|GetDisplayName (Class|GameModeBase|FindPlayerStart _asbp_player_controller (Utilities|Select :Index (Default|GetPlayerType _asbp_player_controller) :EXPLORER "SpawnExplorer" :MUMMY "SpawnMummy"))))
  (return (Class|GameModeBase|FindPlayerStart _asbp_player_controller (Utilities|Select :Index (Default|GetPlayerType _asbp_player_controller) :EXPLORER "SpawnExplorer" :MUMMY "SpawnMummy"))))

(fn DistributeTreasureTiles
  (for _array_element (Variables|Labyrinth|GetTreasure%20Zones)
    (bind _output_get (LocalVariables|SetTreasureTiles (.treasures _array_element)))
    (Utilities|Array|Shuffle _output_get)
    (for (_array_element_2 _array_index) (LocalVariables|GetTreasureTiles)
      (LocalVariables|SetCurrentTileIndex _array_index)
      (bind _asbp_labyrinth_tile (Utilities|Casting|CastToBP_LabyrinthTile _array_element_2))
      (LocalVariables|SetCurrentTile _asbp_labyrinth_tile)
      (Utilities|FlowControl|Sequence
        (:then_0
          (Default|SyncTreasureTile (Variables|Default|GetConnectedMummy) (LocalVariables|GetCurrentTile)))
        (:then_1
          (if (Utilities|Array|IsValidIndex (Variables|Default|GetConnectedExplorers) (LocalVariables|GetCurrentTileIndex))
            (Default|SyncAddTreasureTile (Utilities|Array|Get(acopy) (Variables|Default|GetConnectedExplorers) (LocalVariables|GetCurrentTileIndex)) (LocalVariables|GetCurrentTile))))))))

(fn ConnectPlayer
  (params (PC :type Object%20Object%20Reference))
  (bind _asbp_player_controller (Utilities|Casting|CastToBP_PlayerController PC))
  (bind _output_get (LocalVariables|SetPlayerController _asbp_player_controller))
  (Default|PreInitializeController _output_get)
  (if (Default|IsExplorer _output_get)
    (Utilities|Array|Add (Variables|Default|GetConnectedExplorers) (LocalVariables|GetPlayerController))
    (else
      (Variables|Default|SetConnectedMummy (LocalVariables|GetPlayerController))))
  (Class|KismetSystemLibrary|SetTimerforNextTickDelegate (EventDispatchers|CreateEvent :!event Custom|AttemptStartGame)))

(fn OnPlayerTurn
  (if (and (not (Variables|Turns|GetIs%20Special%20Turn)) (Utilities|Array|IsValidIndex (Variables|Default|GetConnectedExplorers) (Variables|Turns|GetTurnIdx)))
    (Variables|Turns|SetCurrentPlayer (Utilities|Array|Get(acopy) (Variables|Default|GetConnectedExplorers) (Variables|Turns|GetTurnIdx)))
    (Math|Integer|IncrementInt (Variables|Turns|GetTurnIdx)
      (:%20%20
        (Default|SERInitializeTurn (Variables|Turns|GetCurrentPlayer) (Variables|Turns|GetDieValues))))
    (else
      (Variables|Turns|SetCurrentPlayer (Variables|Default|GetConnectedMummy))
      (if (Variables|Turns|GetIs%20Special%20Turn)
        (bind _result (Math|Integer|DecrementInt (Variables|Turns|GetTurnIdx))
          (:%20%20
            (Variables|Turns|SetTurnIdx (Math|Integer|Clamp(Integer) _result 0 (Utilities|Array|LastIndex (Variables|Default|GetConnectedExplorers))))
            (Variables|Turns|SetIs%20Special%20Turn false)
            (Default|SERInitializeSpecialTurn (Variables|Turns|GetCurrentPlayer) (Variables|Turns|GetDieValues))))
        (else
          (Variables|Turns|SetTurnIdx (Math|Integer|%(Integer) (Variables|Turns|GetTurnIdx) (Utilities|Array|Length (Variables|Default|GetConnectedExplorers))))
          (Default|SERInitializeTurn (Variables|Turns|GetCurrentPlayer) (Variables|Turns|GetDieValues))))))
  (EventDispatchers|BindEventtoOnTurnFinished (Variables|Turns|GetCurrentPlayer) (EventDispatchers|CreateEvent :!event Custom|FinishPlayerTurn))
  (EventDispatchers|BindEventtoOnTreasureGrabbed (Variables|Turns|GetCurrentPlayer) (EventDispatchers|CreateEvent :!event NotifyTreasureGrabbed))
  (EventDispatchers|BindEventtoOnExplorerCaught (Variables|Turns|GetCurrentPlayer) (EventDispatchers|CreateEvent :!event NotifyExplorerCaught)))

(fn NotifyTreasureGrabbed
  (params (ZoneIdx :type Integer) (TreasureName :type Text) (PlayerName :type Text))
  (for _array_element (Variables|Default|GetConnectedExplorers)
    (Default|SERNotifyTreasureGrab _array_element ZoneIdx TreasureName PlayerName))
  (Default|SERNotifyTreasureGrab (Variables|Default|GetConnectedMummy) ZoneIdx TreasureName PlayerName))

(fn HasPlayerWon
  (if (Default|IsExplorer (Variables|Turns|GetCurrentPlayer))
    (return (== (Utilities|Array|Length (Variables|/Game/Blueprints/Characters/Player/BP_PlayerController.BP_PlayerController_C|GetTreasureTiles (Variables|Turns|GetCurrentPlayer))) 0))
    (else
      (return (>= (Variables|/Game/Blueprints/Characters/Player/BP_PlayerController.BP_PlayerController_C|GetLives (Variables|Turns|GetCurrentPlayer)) (Utilities|Array|Get(acopy) (Variables|WinConditions|GetMummyWinValues) (- (Variables|WinConditions|GetConnectedExplorersAmount) 1)))))))

(fn NotifyExplorerCaught
  (params (PlayerName :type Text))
  (for _array_element (Variables|Default|GetConnectedExplorers)
    (Default|SERNotifyExplorerCaught _array_element PlayerName))
  (Default|SERNotifyExplorerCaught (Variables|Default|GetConnectedMummy) PlayerName))

(fn DisconnectPlayer
  (params (PlayerController :type Object%20Object%20Reference))
  (bind _asbp_player_controller (Utilities|Casting|CastToBP_PlayerController PlayerController))
  (LocalVariables|SetController _asbp_player_controller)
  (if (Default|IsExplorer _asbp_player_controller)
    (if (> (Variables|/Game/Blueprints/Characters/Player/BP_PlayerController.BP_PlayerController_C|GetLives (LocalVariables|GetController)) 0)
      (Math|Integer|DecrementInt (Variables|WinConditions|GetConnectedExplorersAmount)))))

(fn UpdateClientCollisions
  (for _array_element (Variables|Labyrinth|GetTiles)
    (bind _asbp_labyrinth_tile (Utilities|Casting|CastToBP_LabyrinthTile _array_element))
    (Default|UpdateClientCollisions _asbp_labyrinth_tile)
    (Networking|ForceNetUpdate _asbp_labyrinth_tile)))

(fn PostInitializeControllers
  (for _array_element (Variables|Default|GetConnectedExplorers)
    (Default|PostInitializeController _array_element))
  (Default|PostInitializeController (Variables|Default|GetConnectedMummy))
  (Development|PrintString "Controllers initialized"))

(fn SetExplorersInvisibletoMummy
  (Default|OnHideExplorers (Variables|Default|GetConnectedMummy)))