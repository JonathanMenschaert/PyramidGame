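; Lobby game mode that gathers joining players and launches the multiplayer match.
; PostLogin adds each joining BP_LobbyController to an array.
; StartGame tells one randomly chosen controller to change its player type to MUMMY, then after a short timer runs a listen ServerTravel to L_GameLevel.
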(event Custom|StartGame
  (Default|SERChangePlayerType (Utilities|Array|Get(acopy) (Variables|Default|GetPlayerControllers) (Math|Random|RandomInteger (Utilities|Array|Length (Variables|Default|GetPlayerControllers)))) "MUMMY")
  (Utilities|Time|SetTimerbyEvent (delegate Custom|TravelToServer) 1.0))

(event Custom|TravelToServer
  (Development|ExecuteConsoleCommand "ServerTravel L_GameLevel?Listen" 0))

(event EventPostLogin
  (params (NewPlayer :type Player%20Controller%20Object%20Reference))
  (bind _asbp_lobby_controller (Utilities|Casting|CastToBP_LobbyController NewPlayer))
  (Utilities|Array|Add (Variables|Default|GetPlayerControllers) _asbp_lobby_controller))

(fn ConstructionScript)