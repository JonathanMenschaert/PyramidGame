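; BP_LabyrinthGame is a labyrinth game actor that sizes and positions its floor to fit a generated labyrinth.
; InitializeGameFloor converts the generator result's tile counts and tile size into floor dimensions, and OnUpdateFloorDimensions in the RepLabyrinthGame graph accepts them directly.
; Both feed SetFloorDimensions, which teleports the actor to the center point with half-tile and slight downward offsets, then scales the Floor component.
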(event EventBeginPlay)

(event Collision|EventActorBeginOverlap
  (params (OtherActor :type Actor%20Object%20Reference)))

(event EventTick
  (params (DeltaSeconds :type Float%20%28single-precision%29)))

(event Custom|OnUpdateFloorDimensions
  (params (ScaleX :type Float%20%28single-precision%29) (ScaleY :type Float%20%28single-precision%29) (TileSize :type Float%20%28single-precision%29) (CenterPoint :type Vector))
  (CallFunction|SetFloorDimensions ScaleX ScaleY TileSize CenterPoint))

(fn ConstructionScript)

(fn InitializeGameFloor
  (params (Generator%20Result :type Labyrinth%20Generator%20Result%20Structure))
  (bind (_generatedtiles _sizex _sizey _tilesize _centerpoint) (Utilities|Struct|BreakLabyrinthGeneratorResult Generator%20Result))
  (CallFunction|SetFloorDimensions (* _sizex _tilesize) (* _sizey _tilesize) _tilesize _centerpoint))

(fn SetFloorDimensions
  (params (ScaleX :type Float%20%28single-precision%29) (ScaleY :type Float%20%28single-precision%29) (TileSize :type Float%20%28single-precision%29) (CenterPoint :type Vector))
  (bind _returnvalue (* TileSize 0.5))
  (Transformation|SetActorLocation (- CenterPoint (Math|Vector|MakeVector _returnvalue _returnvalue 1e+01)) false true)
  (Transformation|SetWorldScale3D (Variables|Default|GetFloor) (Math|Vector|MakeVector ScaleX ScaleY 1.0)))