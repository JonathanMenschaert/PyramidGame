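; A single labyrinth tile, hallway or room, that builds its walls and pillars and hosts treasure, torches and spawn points.
; Layout updates reset the tile, add walls on closed sides and pillars except between open rooms, then place torches on even coordinates.
; Treasure attaches to a random eligible side holder, while metadata attaches tagged Explorer or Mummy spawn actors.
; Collision profiles reach clients through OnRep functions and a multicast refresh.
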(event Custom|UpdateClientCollisions
  ;[1 1 1] Properly initialize the collision profiles on the client
  (CallFunction|MULUpdateClientCollisions (Variables|Replication|Collision|GetSWPillarProfile) (Variables|Replication|Collision|GetSEPillarProfile) (Variables|Replication|Collision|GetNEPillarProfile) (Variables|Replication|Collision|GetNWPillarProfile) (Variables|Replication|Collision|GetNorthWallProfile) (Variables|Replication|Collision|GetSouthWallProfile) (Variables|Replication|Collision|GetEastWallProfile) (Variables|Replication|Collision|GetWestWallProfile)))

(event Custom|CLI_SyncTreasure
  (params (Treasure :type BP%20Base%20Treasure%20Object%20Reference) (ZoneIdx :type Integer))
  (bind _output_get (Variables|Treasure|SetTreasure Treasure))
  (Default|SetZoneIndex _output_get ZoneIdx))

(event Custom|MUL_UpdateClientCollisions
  (params (SWPillarProfile :type Name) (SEPillarProfile :type Name) (NEPillarProfile :type Name) (NWPillarProfile :type Name) (NorthWallProfile :type Name) (SouthWallProfile :type Name) (EastWallProfile :type Name) (WestWallProfile :type Name))
  ;[1 1 1] Properly initialize the collision profiles on the client
  (Collision|SetCollisionProfileName (Variables|Default|GetSWPillarCollision) SWPillarProfile true :!class /Script/Engine.PrimitiveComponent)
  (Collision|SetCollisionProfileName (Variables|Default|GetSEPillarCollision) SEPillarProfile true :!class /Script/Engine.PrimitiveComponent)
  (Collision|SetCollisionProfileName (Variables|Default|GetNEPillarCollision) NEPillarProfile true :!class /Script/Engine.PrimitiveComponent)
  (Collision|SetCollisionProfileName (Variables|Default|GetNWPillarCollision) NWPillarProfile true :!class /Script/Engine.PrimitiveComponent)
  (Collision|SetCollisionProfileName (Variables|Default|GetNorthWallCollision) NorthWallProfile true :!class /Script/Engine.PrimitiveComponent)
  (Collision|SetCollisionProfileName (Variables|Default|GetSouthWallCollision) SouthWallProfile true :!class /Script/Engine.PrimitiveComponent)
  (Collision|SetCollisionProfileName (Variables|Default|GetEastWallCollision) EastWallProfile true :!class /Script/Engine.PrimitiveComponent)
  (Collision|SetCollisionProfileName (Variables|Default|GetWestWallCollision) WestWallProfile true :!class /Script/Engine.PrimitiveComponent))

(event EventOnTreasureAdded
  (params (zoneIdx :type Integer) (treasureIdx :type Integer))
  (CallFunction|SpawnTreasure zoneIdx treasureIdx))

(event EventOnTileMetaData
  (params (metaData :type Array%20of%20ETileMetaData%20Enums :default "NONE"))
  (CallFunction|ApplyMetaData metaData))

(event EventUpdateTileDirections
  (params (directions :type Array%20of%20ETileDirection%20Enums :default "NONE") (adjacentTiles :type Map%20of%20ETileDirection%20Enums%20to%20Objects :default "NONE"))
  (CallFunction|UpdateTileLayout directions adjacentTiles))

(fn ConstructionScript)

(fn UpdateTileLayout
  (params (TileDirections :type Array%20of%20ETileDirection%20Enums :default "NONE") (AdjacentTiles :type Map%20of%20ETileDirection%20Enums%20to%20Objects :default "NONE"))
  (CallFunction|ResetTileLayout)
  (bind _enumvalue (|ForEachETileDirection)
    (:LoopBody
      (bind _output_get (LocalVariables|SetCurrentTileDirection _enumvalue))
      (if (Utilities|Array|ContainsItem TileDirections _output_get)
        (if (.ReturnValue (Utilities|Map|Find AdjacentTiles (LocalVariables|GetCurrentTileDirection)))
          (bind _output_get_2 (LocalVariables|SetAdjacentTile (.Value (Utilities|Map|Find AdjacentTiles (LocalVariables|GetCurrentTileDirection)))))
          (if (not (and (Utilities|Enum|Equal(Enum) (Variables|Default|GetTileType) (Variables|/Script/Labyrinth.TileBase|GetTileType _output_get_2)) (Utilities|Enum|Equal(Enum) (Variables|/Script/Labyrinth.TileBase|GetTileType _output_get_2) "ROOM")))
            (CallFunction|UpdateTilePillars (LocalVariables|GetCurrentTileDirection) :!label _label))
          (else
            (goto _label)))
        (else
          (CallFunction|UpdateTileWalls (LocalVariables|GetCurrentTileDirection)))))
    (:then
      (CallFunction|SpawnTorch))))

(fn ApplyMetaData
  (params (Array :type Array%20of%20ETileMetaData%20Enums :default "NONE"))
  (for _array_element Array
    (switch Utilities|FlowControl|Switch|SwitchonETileMetaData _array_element
      (:METAOPTION1
        (bind _outactors (Actor|GetAllActorswithTag "SpawnExplorer"))
        (Transformation|AttachComponentToComponent (Utilities|Array|Get(acopy) _outactors) (Variables|Default|GetRoot) "None" "SnapToTarget" "SnapToTarget" "SnapToTarget" true))
      (:METAOPTION2
        (bind _outactors_2 (Actor|GetAllActorswithTag "SpawnMummy"))
        (Transformation|AttachComponentToComponent (Utilities|Array|Get(acopy) _outactors_2) (Variables|Default|GetRoot) "None" "SnapToTarget" "SnapToTarget" "SnapToTarget" true)))))

(fn UpdateTilePillars
  (params (TileDirection :type ETileDirection%20Enum :default "NONE"))
  (switch Utilities|FlowControl|Switch|SwitchonETileDirection TileDirection
    (:LEFT
      (Rendering|SetVisibility (Variables|Default|GetSWPillar) true true)
      (bind _output_get (Variables|Replication|Collision|SetSWPillarProfile (Variables|Replication|Collision|GetBlockallQueryProfile)))
      (bind _output_get_2 (Variables|Replication|Collision|SetNWPillarProfile _output_get))
      (Collision|SetCollisionProfileName (Variables|Default|GetSWPillarCollision) _output_get_2 true :!class /Script/Engine.PrimitiveComponent))
    (:RIGHT
      (Rendering|SetVisibility (Variables|Default|GetSEPillar) true true)
      (bind _output_get_3 (Variables|Replication|Collision|SetSEPillarProfile (Variables|Replication|Collision|GetBlockallQueryProfile)))
      (bind _output_get_4 (Variables|Replication|Collision|SetNEPillarProfile _output_get_3))
      (Collision|SetCollisionProfileName (Variables|Default|GetSEPillarCollision) _output_get_4 true :!class /Script/Engine.PrimitiveComponent))
    (:UP
      (Rendering|SetVisibility (Variables|Default|GetNEPillar) true true)
      (bind _output_get_5 (Variables|Replication|Collision|SetNEPillarProfile (Variables|Replication|Collision|GetBlockallQueryProfile)))
      (bind _output_get_6 (Variables|Replication|Collision|SetNWPillarProfile _output_get_5))
      (Collision|SetCollisionProfileName (Variables|Default|GetNEPillarCollision) _output_get_6 true :!class /Script/Engine.PrimitiveComponent))
    (:DOWN
      (Rendering|SetVisibility (Variables|Default|GetSWPillar) true true)
      (bind _output_get_7 (Variables|Replication|Collision|SetSWPillarProfile (Variables|Replication|Collision|GetBlockallQueryProfile)))
      (bind _output_get_8 (Variables|Replication|Collision|SetSEPillarProfile _output_get_7))
      (Collision|SetCollisionProfileName (Variables|Default|GetSWPillarCollision) _output_get_8 true :!class /Script/Engine.PrimitiveComponent))))

(fn UpdateTileWalls
  (params (Selection :type ETileDirection%20Enum :default "NONE"))
  (CallFunction|UpdateTilePillars Selection)
  (switch Utilities|FlowControl|Switch|SwitchonETileDirection Selection
    (:LEFT
      (bind _output_get (Variables|Replication|Collision|SetWestWallProfile (Variables|Replication|Collision|GetLabyrinthWallProfile)))
      (Collision|SetCollisionProfileName (Variables|Default|GetWestWallCollision) _output_get true :!class /Script/Engine.PrimitiveComponent)
      (Rendering|SetVisibility (Variables|Default|GetWestWall) true true))
    (:RIGHT
      (bind _output_get_2 (Variables|Replication|Collision|SetEastWallProfile (Variables|Replication|Collision|GetLabyrinthWallProfile)))
      (Collision|SetCollisionProfileName (Variables|Default|GetEastWallCollision) _output_get_2 true :!class /Script/Engine.PrimitiveComponent)
      (Rendering|SetVisibility (Variables|Default|GetEastWall) true true))
    (:UP
      (bind _output_get_3 (Variables|Replication|Collision|SetNorthWallProfile (Variables|Replication|Collision|GetLabyrinthWallProfile)))
      (Collision|SetCollisionProfileName (Variables|Default|GetNorthWallCollision) _output_get_3 true :!class /Script/Engine.PrimitiveComponent)
      (Rendering|SetVisibility (Variables|Default|GetNorthWall) true true))
    (:DOWN
      (bind _output_get_4 (Variables|Replication|Collision|SetSouthWallProfile (Variables|Replication|Collision|GetLabyrinthWallProfile)))
      (Collision|SetCollisionProfileName (Variables|Default|GetSouthWallCollision) _output_get_4 true :!class /Script/Engine.PrimitiveComponent)
      (Rendering|SetVisibility (Variables|Default|GetSouthWall) true true))))

(fn ResetTileLayout
  (bind _output_get (Variables|Replication|Collision|SetSWPillarProfile (Variables|Replication|Collision|GetIgnoreCollisionProfile)))
  (bind _output_get_2 (Variables|Replication|Collision|SetSEPillarProfile _output_get))
  (bind _output_get_3 (Variables|Replication|Collision|SetNEPillarProfile _output_get_2))
  (bind _output_get_4 (Variables|Replication|Collision|SetNWPillarProfile _output_get_3))
  (Collision|SetCollisionProfileName (Variables|Default|GetSWPillarCollision) _output_get_4 true :!class /Script/Engine.PrimitiveComponent)
  (switch Utilities|FlowControl|Switch|SwitchonETileType (Variables|Default|GetTileType)
    (:HALLWAY
      (bind _output_get_5 (Variables|Replication|Collision|SetNorthWallProfile (Variables|Replication|Collision|GetLabyrinthHallwayProfile)))
      (bind _output_get_6 (Variables|Replication|Collision|SetSouthWallProfile _output_get_5))
      (bind _output_get_7 (Variables|Replication|Collision|SetEastWallProfile _output_get_6))
      (bind _output_get_8 (Variables|Replication|Collision|SetWestWallProfile _output_get_7))
      (Collision|SetCollisionProfileName (Variables|Default|GetSouthWallCollision) _output_get_8 true :!class /Script/Engine.PrimitiveComponent))
    (:ROOM
      (bind _output_get_9 (Variables|Replication|Collision|SetNorthWallProfile (Variables|Replication|Collision|GetIgnoreCollisionProfile)))
      (bind _output_get_10 (Variables|Replication|Collision|SetSouthWallProfile _output_get_9))
      (bind _output_get_11 (Variables|Replication|Collision|SetEastWallProfile _output_get_10))
      (bind _output_get_12 (Variables|Replication|Collision|SetWestWallProfile _output_get_11))
      (Collision|SetCollisionProfileName (Variables|Default|GetSouthWallCollision) _output_get_12 true :!class /Script/Engine.PrimitiveComponent)))
  (Rendering|SetVisibility (Variables|Default|GetSouthWall) false true))

(fn OnRepSWPillarProfile
  (Collision|SetCollisionProfileName (Variables|Default|GetSWPillarCollision) (Variables|Replication|Collision|GetSWPillarProfile) true :!class /Script/Engine.PrimitiveComponent))

(fn OnRepSEPillarProfile
  (Collision|SetCollisionProfileName (Variables|Default|GetSEPillarCollision) (Variables|Replication|Collision|GetSEPillarProfile) true :!class /Script/Engine.PrimitiveComponent))

(fn OnRepNEPillarProfile
  (Collision|SetCollisionProfileName (Variables|Default|GetNEPillarCollision) (Variables|Replication|Collision|GetNEPillarProfile) true :!class /Script/Engine.PrimitiveComponent))

(fn OnRepNWPillarProfile
  (Collision|SetCollisionProfileName (Variables|Default|GetNWPillarCollision) (Variables|Replication|Collision|GetNWPillarProfile) true :!class /Script/Engine.PrimitiveComponent))

(fn OnRepNorthWallProfile
  (Collision|SetCollisionProfileName (Variables|Default|GetNorthWallCollision) (Variables|Replication|Collision|GetNorthWallProfile) true :!class /Script/Engine.PrimitiveComponent))

(fn OnRepSouthWallProfile
  (Collision|SetCollisionProfileName (Variables|Default|GetSouthWallCollision) (Variables|Replication|Collision|GetSouthWallProfile) true :!class /Script/Engine.PrimitiveComponent))

(fn OnRepEastWallProfile
  (Collision|SetCollisionProfileName (Variables|Default|GetEastWallCollision) (Variables|Replication|Collision|GetEastWallProfile) true :!class /Script/Engine.PrimitiveComponent))

(fn OnRepWestWallProfile
  (Collision|SetCollisionProfileName (Variables|Default|GetWestWallCollision) (Variables|Replication|Collision|GetWestWallProfile) true :!class /Script/Engine.PrimitiveComponent))

(fn IsValidTile
  (return (Utilities|Enum|Equal(Enum) (Variables|Default|GetTileType) "HALLWAY")))

(fn GetTreasure
  (return (Variables|Treasure|GetTreasure)))

(fn SpawnTreasure
  (params (ZoneIdx :type Integer) (TreasureIdx :type Integer))
  (bind _returnvalue (Class|TileBase|GetTreasureDirections))
  (bind _westitemholder (Variables|Default|GetWestItemHolder))
  (if (Utilities|Array|IsValidIndex (Variables|Treasure|GetTreasureClasses) TreasureIdx)
    (Variables|Treasure|SetTreasureDirections _returnvalue)
    (if (> (Utilities|Array|Length _returnvalue) 0)
      (bind _returnvalue_2 (Game|SpawnActorfromClass (Utilities|Array|Get(acopy) (Variables|Treasure|GetTreasureClasses) TreasureIdx) (Transformation|GetActorTransform) "AlwaysSpawn" "MultiplyWithRoot" 0 ZoneIdx 0))
      (bind _output_get (Variables|Treasure|SetTreasure _returnvalue_2))
      (Transformation|AttachComponentToComponent _output_get (Utilities|Select :Index (Utilities|Array|Get(acopy) (Variables|Treasure|GetTreasureDirections) (Math|Random|RandomInteger (Utilities|Array|Length (Variables|Treasure|GetTreasureDirections)))) :NONE _westitemholder :LEFT _westitemholder :RIGHT (Variables|Default|GetEastItemHolder) :UP (Variables|Default|GetNorthItemHolder) :DOWN (Variables|Default|GetSouthItemHolder)) "None" "SnapToTarget" "SnapToTarget" "KeepWorld" true))))

(fn ActivateTreasure
  (params (Activate :type Boolean))
  (bind _treasure (Variables|Treasure|GetTreasure)
    (:then
      (Variables|/Game/Blueprints/Treasures/BP_BaseTreasure.BP_BaseTreasure_C|SetActivated _treasure Activate))
    (:else)))

(fn SpawnTorch
  (bind _returnvalue (Class|TileBase|GetTreasureDirections))
  (bind _westtorchholder (Variables|Default|GetWestTorchHolder))
  (if (and (== (Math|Integer|%(Integer) (Variables|Default|GetCoordinateX) 2) 0) (== (Math|Integer|%(Integer) (Variables|Default|GetCoordinateY) 2) 0))
    (Variables|Treasure|SetTreasureDirections _returnvalue)
    (if (> (Utilities|Array|Length _returnvalue) 0)
      (bind _returnvalue_2 (Game|SpawnActorfromClass "/Game/Blueprints/Labyrinth/Torch/BP_Torch.BP_Torch_C" (Transformation|GetActorTransform) "AlwaysSpawn" "MultiplyWithRoot" 0 0))
      (Transformation|AttachComponentToComponent _returnvalue_2 (Utilities|Select :Index (Utilities|Array|Get(acopy) (Variables|Treasure|GetTreasureDirections) (Math|Random|RandomInteger (Utilities|Array|Length (Variables|Treasure|GetTreasureDirections)))) :NONE _westtorchholder :LEFT _westtorchholder :RIGHT (Variables|Default|GetEastTorchHolder) :UP (Variables|Default|GetNorthTorchHolder) :DOWN (Variables|Default|GetSouthTorchHolder)) "None" "SnapToTarget" "SnapToTarget" "KeepWorld" true))))