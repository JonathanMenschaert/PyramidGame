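; BP_LabyrinthMovingWall is an interactable labyrinth wall that works as a timed door.
; At BeginPlay it snaps its collision root to the Door component's Wall socket, so collision follows the wall.
; Interacting while closed switches DoorState and starts a one-shot timer that returns it to closed a few seconds later.
; Interaction is always allowed but ignored in the other state, and the graph only sets the state, with no movement logic.
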(event Custom|OnDoorClose
  (Variables|Default|SetDoorState "NewEnumerator1"))

(event EventBeginPlay
  (Transformation|AttachComponentToComponent (Variables|Default|GetCollisionRoot) (Variables|Default|GetDoor) "Wall" "SnapToTarget" "SnapToTarget" "KeepWorld" true))

(event Collision|EventActorBeginOverlap
  (params (OtherActor :type Actor%20Object%20Reference)))

(event EventTick
  (params (DeltaSeconds :type Float%20%28single-precision%29)))

(event EventOnInteract
  (if (Utilities|Enum|Equal(Enum) (Variables|Default|GetDoorState) "NewEnumerator1")
    (Variables|Default|SetDoorState "NewEnumerator0")
    (Utilities|Time|SetTimerbyEvent (delegate Custom|OnDoorClose) 6.0)))

(fn ConstructionScript)

(fn AllowsInteraction
  (return true))