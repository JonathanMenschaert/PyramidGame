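; BP_LabyrinthTile is a labyrinth tile that shows walls and corner pillars to match its set of open directions.
; The UpdateTileDirections event passes the directions to UpdateTileLayout, which first hides every wall and pillar.
; It then loops over the ETileDirection enum and, for each direction missing from the set, reveals that side's wall and its two adjoining pillars.
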(event EventUpdateTileDirections
  (params (directions :type Array%20of%20ETileDirection%20Enums :default "NONE"))
  (CallFunction|UpdateTileLayout directions))

(fn ConstructionScript)

(fn UpdateTileLayout
  (params (TileDirections :type Array%20of%20ETileDirection%20Enums :default "NONE"))
  (Rendering|SetVisibility (Variables|Default|GetSouthWall) false true)
  (bind _enumvalue (|ForEachETileDirection)
    (:LoopBody
      (if (not (Utilities|Array|ContainsItem TileDirections _enumvalue))
        (switch Utilities|FlowControl|Switch|SwitchonETileDirection _enumvalue
          (:LEFT
            (Rendering|SetVisibility (Variables|Default|GetWestWall) true true))
          (:RIGHT
            (Rendering|SetVisibility (Variables|Default|GetEastWall) true true))
          (:UP
            (Rendering|SetVisibility (Variables|Default|GetNorthWall) true true))
          (:DOWN
            (Rendering|SetVisibility (Variables|Default|GetSouthWall) true true)))))))