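; Player controller for a networked, turn-based dice board game in which explorers hunt treasure and mummies catch them.
; The server rolls dice and clients show them; chosen values become steps, spent per tile, with collision profiles gating movement.
; It tracks lives and treasure tiles, retrying client tile sync when the treasure is invalid.
; It also manages the top-view camera, HUD, map, notebook and notifications, swapping input mapping contexts per mode.
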(event Custom|SER_NotifyTreasureGrab
  (params (ZoneIdx :type Integer) (TreasureName :type Text) (PlayerName :type Text))
  ;[1 1 1] Notifications
  (CallFunction|CLINotifyTreasureGrab ZoneIdx TreasureName PlayerName))

(event Custom|CLI_NotifyTreasureGrab
  (params (ZoneIdx :type Integer) (TreasureName :type Text) (PlayerName :type Text))
  ;[1 1 1] Notifications
  (bind _returnvalue (UserInterface|CreateWidget "/Game/UserInterface/Widgets/HUD/WBP_TreasureGrabNotification.WBP_TreasureGrabNotification_C" 0 ZoneIdx TreasureName PlayerName))
  (UserInterface|Viewport|AddtoViewport _returnvalue 0))

(event Custom|SER_RequestResyncAdd
  (params (TreasureTile :type BP%20Labyrinth%20Tile%20Object%20Reference))
  ;[1 1 1] SyncTreasure
  (Utilities|FlowControl|Delay 1.0)
  (Treasure|SyncAddTreasureTile TreasureTile))

(event Custom|SER_RequestResync
  (params (TreasureTile :type BP%20Labyrinth%20Tile%20Object%20Reference))
  ;[1 1 1] SyncTreasure
  (Utilities|FlowControl|Delay 1.0)
  (Treasure|SyncTreasureTile TreasureTile))

(event Custom|SER_NotifyExplorerCaught
  (params (PlayerName :type Text))
  ;[1 1 1] Notifications
  (CallFunction|CLINotifyExplorerCaught PlayerName))

(event Custom|CLI_NotifyExplorerCaught
  (params (PlayerName :type Text))
  ;[1 1 1] Notifications
  (bind _returnvalue (UserInterface|CreateWidget "/Game/UserInterface/Widgets/HUD/WBP_ExplorerCaughtNotification.WBP_ExplorerCaughtNotification_C" 0 PlayerName))
  (UserInterface|Viewport|AddtoViewport _returnvalue 0))

(event Custom|CLI_SyncTreasureTile
  (params (TreasureTile :type BP%20Labyrinth%20Tile%20Object%20Reference) (Treasure :type BP%20Base%20Treasure%20Object%20Reference) (ZoneIdx :type Integer))
  ;[1 1 1] SyncTreasure
  (Utilities|IsValid Treasure
    (:Is%20Valid
      (Default|CLISyncTreasure TreasureTile Treasure ZoneIdx))
    (:Is%20Not%20Valid
      (CallFunction|SERRequestResync TreasureTile))))

(event Custom|PostInitializeController
  ;[1 1 1] Initialize
  (CallFunction|CLIPostInitializeController)
  (Turn|InitializeLives)
  (CallFunction|CLIonUpdateLives (Variables|Default|GetLives))
  (Turn|UpdateSteps)
  (CallFunction|CLIonUpdateSteps (Variables|Default|GetPlayerSteps)))

(event Custom|CLI_SyncAddTreasureTile
  (params (TreasureTile :type BP%20Labyrinth%20Tile%20Object%20Reference) (Treasure :type BP%20Base%20Treasure%20Object%20Reference) (ZoneIdx :type Integer))
  ;[1 1 1] SyncTreasure
  (Utilities|IsValid Treasure
    (:Is%20Valid
      (Default|CLISyncTreasure TreasureTile Treasure ZoneIdx)
      (Treasure|AddTreasureTile TreasureTile))
    (:Is%20Not%20Valid
      (CallFunction|SERRequestResyncAdd TreasureTile))))

(event Custom|CLI_PostInitializeController
  ;[1 1 1] Initialize
  (Widget|RemovefromParent (Variables|Widgets|GetLoadingScreen))
  (General|RestoreIMC)
  (Input|SetInputModeGameOnly self true)
  (UserInterface|Viewport|AddtoViewport (Variables|Default|GetPlayerHud) 0))

(event Custom|CLI_PreInitializeController
  ;[1 1 1] Initialize
  (bind _returnvalue (UserInterface|CreateWidget "/Game/UserInterface/Widgets/Menu/WBP_LoadingScreen.WBP_LoadingScreen_C"))
  (UserInterface|Viewport|AddtoViewport _returnvalue 0)
  (Variables|Widgets|SetLoadingScreen _returnvalue)
  (Input|SetInputModeUIOnly self _returnvalue "DoNotLock" true))

(event Custom|PreInitializeController
  ;[1 1 1] Initialize
  (CallFunction|CLIPreInitializeController))

(event Input|EnhancedActionEvents|EnhancedInputActionIA_OpenMap
  (params (ActionValue :type Boolean) (ElapsedSeconds :type Float%20%28double-precision%29) (TriggeredSeconds :type Float%20%28double-precision%29) (InputAction :type Input%20Action%20Object%20Reference :default "/Game/Blueprints/Characters/Player/Input/Actions/IA_OpenMap.IA_OpenMap"))
  ;[1 1 1] UIControl
  (:Started
    (if (Pawn|IsLocallyControlled (Variables|Default|GetControlledPawn))
      (bind _returnvalue (UserInterface|CreateWidget "/Game/UserInterface/Widgets/Map/WBP_Map.WBP_Map_C" self))
      (Variables|Widgets|SetActiveUI _returnvalue)
      (General|SwapMappingContext)
      (Default|OpenMap (Variables|Default|GetControlledPawn)))))

(event Input|EnhancedActionEvents|EnhancedInputActionIA_CloseUI
  (params (ActionValue :type Boolean) (ElapsedSeconds :type Float%20%28double-precision%29) (TriggeredSeconds :type Float%20%28double-precision%29) (InputAction :type Input%20Action%20Object%20Reference :default "/Game/Blueprints/Characters/Player/Input/Actions/IA_CloseUI.IA_CloseUI"))
  ;[1 1 1] UIControl
  (:Started
    (if (Pawn|IsLocallyControlled (Variables|Default|GetControlledPawn))
      (Default|CloseUI (Variables|Default|GetControlledPawn)))))

(event Input|EnhancedActionEvents|EnhancedInputActionIA_OpenNotebook
  (params (ActionValue :type Boolean) (ElapsedSeconds :type Float%20%28double-precision%29) (TriggeredSeconds :type Float%20%28double-precision%29) (InputAction :type Input%20Action%20Object%20Reference :default "/Game/Blueprints/Characters/Player/Input/Actions/IA_OpenNotebook.IA_OpenNotebook"))
  ;[1 1 1] UIControl
  (if (Pawn|IsLocallyControlled (Variables|Default|GetControlledPawn))
    (bind _returnvalue (UserInterface|CreateWidget "/Game/UserInterface/Widgets/Notebook/WBP_Itemlog.WBP_Itemlog_C" self))
    (Default|InitializeNotebook _returnvalue (Variables|Default|GetTreasureTiles))
    (Variables|Widgets|SetActiveUI _returnvalue)
    (General|SwapMappingContext)
    (Default|OpenBook (Variables|Default|GetControlledPawn))))

(event Input|EnhancedActionEvents|EnhancedInputActionIA_MoveMapCamera
  (params (ActionValue :type Vector%202D%20Structure) (ElapsedSeconds :type Float%20%28double-precision%29) (TriggeredSeconds :type Float%20%28double-precision%29) (InputAction :type Input%20Action%20Object%20Reference :default "/Game/Blueprints/Characters/Player/Input/Actions/IA_MoveMapCamera.IA_MoveMapCamera"))
  (bind _returnvalue (Utilities|Time|GetWorldDeltaSeconds))
  (bind _viewcamera (Variables|Map|GetViewCamera))
  (bind _returnvalue_2 (Transformation|GetActorLocation _viewcamera))
  ;[1 1 1] UIControl
  (Transformation|SetActorLocation (Variables|Map|GetViewCamera) (Math|Vector|MakeVector (+ (* (Variables|Map|GetCameraMovementSpeed) (.y ActionValue) _returnvalue) (.x _returnvalue_2)) (+ (* (Variables|Map|GetCameraMovementSpeed) (.x ActionValue) _returnvalue) (.y _returnvalue_2)) (.z _returnvalue_2)) false true))

(event EventBeginPlay
  ;[1 1 1] Set up Controller
  (Utilities|FlowControl|Delay 1.0)
  (bind _asbp_player_character (Utilities|Casting|CastToBP_PlayerCharacter (Pawn|GetControlledPawn)))
  (bind _output_get (Variables|Default|SetControlledPawn _asbp_player_character))
  (EventDispatchers|AssignOnTileEntered _output_get (EventDispatchers|CreateEvent :!event Custom|OnTileEntered))
  (EventDispatchers|BindEventtoOnCaughtbyMummy (Variables|Default|GetControlledPawn) (EventDispatchers|CreateEvent :!event OnCaughtbyMummy))
  (if (Pawn|IsLocallyControlled (Variables|Default|GetControlledPawn))
    (EventDispatchers|BindEventtoOnUIClosed (Variables|Default|GetControlledPawn) (EventDispatchers|CreateEvent :!event RestoreIMC))
    (EventDispatchers|BindEventtoOnUIStartClosing (Variables|Default|GetControlledPawn) (EventDispatchers|CreateEvent :!event RemoveUI))
    (EventDispatchers|BindEventtoOnUIOpened (Variables|Default|GetControlledPawn) (EventDispatchers|CreateEvent :!event AttachUI))
    (bind _returnvalue (Game|SpawnActorfromClass "/Game/Blueprints/Items/Map/BP_TopViewCamera.BP_TopViewCamera_C" (Transformation|GetActorTransform (Variables|Default|GetControlledPawn)) "AlwaysSpawn" "MultiplyWithRoot" 0 (Variables|Default|GetControlledPawn) 0))
    (bind _output_get_2 (Variables|Map|SetViewCamera _returnvalue))
    (Transformation|AttachActorToActor _output_get_2 (Variables|Default|GetControlledPawn) "None" "SnapToTarget" "SnapToTarget" "SnapToTarget" true)
    (bind _returnvalue_2 (UserInterface|CreateWidget "/Game/UserInterface/Widgets/HUD/WBP_HUD.WBP_HUD_C"))
    (Variables|Default|SetPlayerHud _returnvalue_2)))

(event Custom|SER_InitializeTurn
  (params (DieValues :type Array%20of%20Integers))
  ;[1 1 1] Control Turn
  (bind _output_get (Variables|Dice|SetDieValues DieValues))
  (Turn|UpdateSteps)
  (CallFunction|CLIInitializeTurn _output_get))

(event Custom|OnTileEntered
  (params (Tile :type BP%20Labyrinth%20Tile%20Object%20Reference))
  ;[1 1 1] Control Turn
  (Treasure|ResetPreviousTile)
  (bind _output_get (Variables|Default|SetCurrentTile Tile))
  (Treasure|ActivateTreasureTile _output_get)
  (bind _result (Math|Integer|DecrementInt (Variables|Default|GetPlayerSteps))
    (:%20%20
      (Turn|UpdateSteps _result)
      (if (> (Variables|Default|GetPlayerSteps) 0)
        (Development|PrintString (Utilities|String|ToString(Integer) (Variables|Default|GetPlayerSteps)))
        (else
          (CallFunction|SetCollisiontoIdle))))))

(event Custom|SER_RollDice
  ;[1 1 1] Rolling dice
  (if (General|IsExplorer)
    (Dice|RollExplorerDice)
    (CallFunction|CLIRollDiceExplorer (Variables|Dice|GetDieValues))
    (else
      (Dice|HandleMummyDice))))

(event Custom|CLI_RollDiceExplorer
  (params (DieValues :type Array%20of%20Integers))
  ;[1 1 1] Rolling dice
  (bind _output_get (Variables|Dice|SetDieValues DieValues))
  (Default|UpdateDice (Variables|Dice|GetDiceHolder) _output_get)
  (Utilities|FlowControl|Delay 1.5)
  (Default|StopRolling (Variables|Dice|GetDiceHolder))
  (Utilities|FlowControl|Delay 1.5)
  (Default|AllowDiceSelection (Variables|Dice|GetDiceHolder) true)
  (Variables|Dice|SetCanReroll true))

(event Custom|SetCollisionToIdle
  ;[1 1 1] Control Turn
  (Default|OnTurnEnd (Variables|Default|GetControlledPawn))
  (Default|UpdateCollisionProfile (Variables|Default|GetControlledPawn)))

(event Custom|StartRollingDice
  ;[1 1 1] Rolling dice
  (Default|AllowDiceSelection (Variables|Dice|GetDiceHolder) false)
  (Default|StartRolling (Variables|Dice|GetDiceHolder))
  (CallFunction|SERRollDice))

(event Custom|CLI_RollDiceMummy
  (params (ExtraSteps :type Integer) (DieValue :type Integer))
  ;[1 1 1] Rolling dice
  (Turn|UpdateSteps ExtraSteps)
  (Default|UpdateDice (Variables|Dice|GetDiceHolder) (Utilities|Array|MakeArray DieValue))
  (Utilities|FlowControl|Delay 1.5)
  (Default|StopRolling (Variables|Dice|GetDiceHolder))
  (Utilities|FlowControl|Delay 1.5)
  (Default|AllowDiceSelection (Variables|Dice|GetDiceHolder) true)
  (Variables|Dice|SetCanReroll false))

(event Custom|ForceEndTurn
  ;[1 1 1] Control Turn
  (Turn|UpdateSteps)
  (CallFunction|SetCollisiontoIdle)
  (CallFunction|SEREndTurn false))

(event Custom|CLI_OnUpdateLives
  (params (CurrentLivesAmount :type Integer))
  ;[1 1 1] Handle Lives & Steps Counter
  (Turn|UpdateLives CurrentLivesAmount))

(event Custom|CLI_OnUpdateSteps
  (params (Steps :type Integer))
  ;[1 1 1] Handle Lives & Steps Counter
  (Turn|UpdateSteps Steps))

(event Custom|CLI_InitializeSpecialTurn
  (params (PlayerSteps :type Integer))
  ;[1 1 1] Control Turn
  (Turn|UpdateSteps PlayerSteps)
  (General|SwapMappingContext)
  (bind _returnvalue (UserInterface|CreateWidget "/Game/UserInterface/Widgets/HUD/WBP_YourTurn.WBP_YourTurn_C"))
  (bind _output_get (Variables|Widgets|SetYourTurnScreen _returnvalue))
  (UserInterface|Viewport|AddtoViewport _output_get 0)
  (Utilities|FlowControl|Delay 3.0)
  (Widget|RemovefromParent (Variables|Widgets|GetYourTurnScreen))
  (CallFunction|SetCollisiontoMoving)
  (General|SwapMappingContext "/Game/Blueprints/Characters/Player/Input/IMC_Explorer.IMC_Explorer")
  (Variables|Default|SetIsTurn true))

(event Custom|SER_UpdatePlayerSteps
  (params (PlayerSteps :type Integer))
  ;[1 1 1] Rolling dice
  (Turn|UpdateSteps PlayerSteps)
  (CallFunction|SetCollisiontoMoving))

(event Custom|SetCollisionToMoving
  ;[1 1 1] Control Turn
  (Default|OnTurnStart (Variables|Default|GetControlledPawn))
  (Default|UpdateCollisionProfile (Variables|Default|GetControlledPawn)))

(event Custom|SER_EndTurn
  (params (RequestSpecialTurn :type Boolean))
  ;[1 1 1] Control Turn
  (Turn|UpdateSteps)
  (CallFunction|SetCollisiontoIdle)
  (Default|CallOnTurnFinished RequestSpecialTurn))

(event Custom|SER_InitializeSpecialTurn
  (params (DieValues :type Array%20of%20Integers))
  ;[1 1 1] Control Turn
  (Variables|Dice|SetDieValues DieValues)
  (bind _extrasteps (Dice|ResetExplorerDice))
  (Turn|UpdateSteps _extrasteps)
  (CallFunction|CLIInitializeSpecialTurn (Variables|Default|GetPlayerSteps))
  (Utilities|FlowControl|Delay 3.0)
  (CallFunction|SetCollisiontoMoving))

(event Custom|CLI_InitializeTurn
  (params (DieValues :type Array%20of%20Integers))
  ;[1 1 1] Control Turn
  (Variables|Dice|SetDieValues DieValues)
  (Turn|UpdateSteps)
  (bind _returnvalue (UserInterface|CreateWidget "/Game/UserInterface/Widgets/HUD/WBP_YourTurn.WBP_YourTurn_C"))
  (bind _output_get (Variables|Widgets|SetYourTurnScreen _returnvalue))
  (UserInterface|Viewport|AddtoViewport _output_get 0)
  (Utilities|FlowControl|Delay 3.0)
  (Widget|RemovefromParent (Variables|Widgets|GetYourTurnScreen))
  (Dice|SpawnDiceMenu)
  (Dice|SpawnMouseCursor))

(event Input|EnhancedActionEvents|EnhancedInputActionIA_MouseHover
  (params (ActionValue :type Vector%202D%20Structure) (ElapsedSeconds :type Float%20%28double-precision%29) (TriggeredSeconds :type Float%20%28double-precision%29) (InputAction :type Input%20Action%20Object%20Reference :default "/Game/Blueprints/Characters/Player/Input/Actions/IA_MouseHover.IA_MouseHover"))
  ;[1 1 1] Rolling dice
  (Dice|HoverObject)
  (Dice|UpdateMousePosition))

(event Input|EnhancedActionEvents|EnhancedInputActionIA_Reroll
  (params (ActionValue :type Boolean) (ElapsedSeconds :type Float%20%28double-precision%29) (TriggeredSeconds :type Float%20%28double-precision%29) (InputAction :type Input%20Action%20Object%20Reference :default "/Game/Blueprints/Characters/Player/Input/Actions/IA_Reroll.IA_Reroll"))
  ;[1 1 1] Rolling dice
  (:Started
    (if (Variables|Dice|GetCanReroll)
      (Variables|Dice|SetCanReroll false)
      (CallFunction|StartRollingDice))))

(event Input|EnhancedActionEvents|EnhancedInputActionIA_MouseInteract
  (params (ActionValue :type Boolean) (ElapsedSeconds :type Float%20%28double-precision%29) (TriggeredSeconds :type Float%20%28double-precision%29) (InputAction :type Input%20Action%20Object%20Reference :default "/Game/Blueprints/Characters/Player/Input/Actions/IA_MouseInteract.IA_MouseInteract"))
  ;[1 1 1] Rolling dice
  (:Started
    (Variables|Dice|SetCanReroll false)
    (bind _selecteddievalue (Default|FindSelectedDieValue (Variables|Dice|GetDiceHolder)))
    (if (> _selecteddievalue 0)
      (Turn|UpdateSteps (+ _selecteddievalue (Variables|Default|GetPlayerSteps)))
      (Development|PrintString (Utilities|String|ToString(Integer) (Variables|Default|GetPlayerSteps)))
      (Utilities|FlowControl|Delay 0.2)
      (Dice|RemoveDiceScreen)
      (CallFunction|SERUpdatePlayerSteps (Variables|Default|GetPlayerSteps))
      (CallFunction|SetCollisiontoMoving)
      (Variables|Default|SetIsTurn true))))

(event Input|EnhancedActionEvents|EnhancedInputActionIA_EndTurn
  (params (ActionValue :type Boolean) (ElapsedSeconds :type Float%20%28double-precision%29) (TriggeredSeconds :type Float%20%28double-precision%29) (InputAction :type Input%20Action%20Object%20Reference :default "/Game/Blueprints/Characters/Player/Input/Actions/IA_EndTurn.IA_EndTurn"))
  ;[1 1 1] Control Turn
  (:Started
    (if (Variables|Default|GetIsTurn)
      (Variables|Default|SetIsTurn false)
      (CallFunction|SetCollisiontoIdle)
      (CallFunction|SEREndTurn false)
      (Turn|UpdateSteps))))

(event Input|EnhancedActionEvents|EnhancedInputActionIA_RequestSpecialTurn
  (params (ActionValue :type Boolean) (ElapsedSeconds :type Float%20%28double-precision%29) (TriggeredSeconds :type Float%20%28double-precision%29) (InputAction :type Input%20Action%20Object%20Reference :default "/Game/Blueprints/Characters/Player/Input/Actions/IA_RequestSpecialTurn.IA_RequestSpecialTurn"))
  ;[1 1 1] Control Turn
  (:Started
    (if (Variables|Dice|GetCanReroll)
      (Variables|Default|SetIsTurn false)
      (Dice|RemoveDiceScreen)
      (CallFunction|SetCollisiontoIdle)
      (CallFunction|SEREndTurn true)
      (Turn|UpdateSteps))))

(fn ConstructionScript)

(fn SwapMappingContext
  (params (MappingContext :type Input%20Mapping%20Context%20Object%20Reference))
  (bind _returnvalue (PlayerController|LocalPlayerSubsystems|GetEnhancedInputLocalPlayerSubsystem))
  (Class|EnhancedInputSubsystemInterface|ClearAllMappings _returnvalue)
  (Utilities|IsValid MappingContext
    (:Is%20Valid
      (Input|AddMappingContext _returnvalue MappingContext 0 "(bIgnoreAllPressedKeysUntilRelease=True,bForceImmediately=False,bNotifyUserSettings=False)"))))

(fn RestoreIMC
  (if (General|IsExplorer)
    (General|SwapMappingContext "/Game/Blueprints/Characters/Player/Input/IMC_Explorer.IMC_Explorer")
    (else
      (General|SwapMappingContext "/Game/Blueprints/Characters/Player/Input/IMC_Mummy.IMC_Mummy"))))

(fn GetPlayerType
  (bind _asbp_player_state (Utilities|Casting|CastToBP_PlayerState (Variables|Default|GetPlayerState)))
  (return (Variables|/Script/PyramidGame.PlayerStateLabyrinth|GetPlayerType _asbp_player_state)))

(fn AddTreasureTile
  (params (Tile :type BP%20Labyrinth%20Tile%20Object%20Reference))
  (Utilities|Array|Add (Variables|Default|GetTreasureTiles) Tile))

(fn IsExplorer
  (bind _asbp_player_state (Utilities|Casting|CastToBP_PlayerState (Variables|Default|GetPlayerState)))
  (return (Utilities|Enum|Equal(Enum) (Variables|/Script/PyramidGame.PlayerStateLabyrinth|GetPlayerType _asbp_player_state) "EXPLORER")))

(fn SyncAddTreasureTile
  (params (TreasureTile :type BP%20Labyrinth%20Tile%20Object%20Reference))
  (bind _treasure (Default|GetTreasure TreasureTile))
  (Treasure|AddTreasureTile TreasureTile)
  (CallFunction|CLISyncAddTreasureTile TreasureTile _treasure (Variables|/Game/Blueprints/Treasures/BP_BaseTreasure.BP_BaseTreasure_C|GetZoneIdx _treasure)))

(fn SyncTreasureTile
  (params (TreasureTile :type BP%20Labyrinth%20Tile%20Object%20Reference))
  (bind _treasure (Default|GetTreasure TreasureTile))
  (CallFunction|CLISyncTreasureTile TreasureTile _treasure (Variables|/Game/Blueprints/Treasures/BP_BaseTreasure.BP_BaseTreasure_C|GetZoneIdx _treasure)))

(fn AttachUI
  (bind _activeui (Variables|Widgets|GetActiveUI)
    (:then
      (UserInterface|Viewport|AddtoViewport _activeui 0)
      (General|SwapMappingContext "/Game/Blueprints/Characters/Player/Input/IMC_UserInterface.IMC_UserInterface"))
    (:else)))

(fn RemoveUI
  (bind _activeui (Variables|Widgets|GetActiveUI)
    (:then
      (Widget|RemovefromParent _activeui)
      (Variables|Widgets|SetActiveUI 0))
    (:else)))

(fn RollExplorerDice
  (for _array_element (Variables|Dice|GetDieValues)
    (if (> _array_element 0)
      (Utilities|Array|Add (LocalVariables|GetCurrentDieValues) (Math|Random|RandomIntegerinRange 0 5))
      (else
        (Utilities|Array|Add (LocalVariables|GetCurrentDieValues) _array_element))))
  (Variables|Dice|SetDieValues (LocalVariables|GetCurrentDieValues)))

(fn ResetExplorerDice
  (for _array_element (Variables|Dice|GetDieValues)
    (if (<= _array_element 0)
      (Math|Integer|IncrementInt (LocalVariables|GetExtraMoves))))
  (Variables|Dice|SetDieValues (LocalVariables|GetNewDie))
  (return (LocalVariables|GetExtraMoves)))

(fn HoverObject
  (bind _output_get (LocalVariables|SetHitActor (.HitActor (Collision|BreakHitResult (.HitResult (Class|PlayerController|GetHitResultUnderCursorforObjects (Utilities|Array|MakeArray "ObjectTypeQuery11") true))))))
  (Utilities|IsValid _output_get
    (:Is%20Valid
      (bind _output_get_2 (Variables|Dice|SetHoverActor (LocalVariables|GetHitActor)))
      (Class|InteractionInterface|OnHoverEnter(Message) _output_get_2))
    (:Is%20Not%20Valid
      (bind _hoveractor (Variables|Dice|GetHoverActor)
        (:then
          (Class|InteractionInterface|OnHoverExit(Message) _hoveractor)
          (Variables|Dice|SetHoverActor 0))
        (:else)))))

(fn UpdateMousePosition
  (bind _self self)
  (bind (_locationx _locationy) (Class|WidgetLayoutLibrary|GetMousePositionScaledbyDPI _self))
  (Class|UserWidget|SetPositioninViewport (Variables|Dice|GetMouseCursor) (Math|Vector2D|MakeVector2D _locationx _locationy) false))

(fn SpawnDiceMenu
  (bind _returnvalue (Game|SpawnActorfromClass "/Game/Blueprints/Items/Dice/BP_DiceHolder.BP_DiceHolder_C" (Transformation|GetActorTransform (Variables|Default|GetControlledPawn)) "AlwaysSpawn" "MultiplyWithRoot" 0 0))
  (Variables|Dice|SetDiceHolder _returnvalue)
  (if (General|IsExplorer)
    (Default|AddDiceScreen (Variables|Default|GetControlledPawn) (Variables|Dice|GetDiceHolder) true)
    (General|SwapMappingContext "/Game/Blueprints/Characters/Player/Input/IMC_ExplorerDiceInterface.IMC_ExplorerDiceInterface")
    (else
      (Default|AddDiceScreen (Variables|Default|GetControlledPawn) (Variables|Dice|GetDiceHolder) false)
      (General|SwapMappingContext "/Game/Blueprints/Characters/Player/Input/IMC_MummyDiceInterface.IMC_MummyDiceInterface")))
  (bind _returnvalue_2 (UserInterface|CreateWidget "/Game/UserInterface/Widgets/Dice/WBP_DiceScreen.WBP_DiceScreen_C"))
  (bind _output_get (Variables|Dice|SetDiceScreen _returnvalue_2))
  (UserInterface|Viewport|AddtoViewport _output_get 0)
  (Variables|Dice|SetCanReroll true)
  (Default|ForceStopRolling (Variables|Dice|GetDiceHolder) (Variables|Dice|GetDieValues)))

(fn SpawnMouseCursor
  (bind _returnvalue (UserInterface|CreateWidget "/Game/UserInterface/Widgets/Menu/WBP_MouseCursor.WBP_MouseCursor_C"))
  (bind _output_get (Variables|Dice|SetMouseCursor _returnvalue))
  (UserInterface|Viewport|AddtoViewport _output_get 0)
  (Dice|UpdateMousePosition))

(fn RemoveDiceScreen
  (General|SwapMappingContext "/Game/Blueprints/Characters/Player/Input/IMC_Explorer.IMC_Explorer")
  (Variables|Dice|SetHoverActor 0)
  (Widget|RemovefromParent (Variables|Dice|GetMouseCursor))
  (Variables|Dice|SetMouseCursor 0)
  (Widget|RemovefromParent (Variables|Dice|GetDiceScreen))
  (Variables|Dice|SetDiceScreen 0)
  (Default|DestroyDice (Variables|Dice|GetDiceHolder))
  (Actor|DestroyActor (Variables|Dice|GetDiceHolder))
  (Variables|Dice|SetDiceHolder 0)
  (Variables|Dice|SetCanReroll false))

(fn ActivateTreasureTile
  (params (Tile :type BP%20Labyrinth%20Tile%20Object%20Reference))
  (bind _output_get (LocalVariables|SetCurrentTileIdx (Utilities|Array|FindItem (Variables|Default|GetTreasureTiles) Tile)))
  (if (>= _output_get 0)
    (Variables|Default|SetActivatedTileIdx (LocalVariables|GetCurrentTileIdx))
    (Default|ActivateTreasure Tile true)
    (EventDispatchers|BindEventtoOnTreasureGrabbed (Variables|/Game/Blueprints/Labyrinth/Tile/BP_LabyrinthTile.BP_LabyrinthTile_C|GetTreasure Tile) (EventDispatchers|CreateEvent :!event RemoveTreasureTile))))

(fn RemoveTreasureTile
  (params (ZoneIdx :type Integer) (TreasureName :type Text))
  (Utilities|Array|RemoveIndex (Variables|Default|GetTreasureTiles) (Variables|Default|GetActivatedTileIdx))
  (Variables|Default|SetActivatedTileIdx -1)
  (Default|CallOnTreasureGrabbed ZoneIdx TreasureName (General|GetPlayerName))
  (CallFunction|ForceEndTurn))

(fn ResetPreviousTile
  (bind _currenttile (Variables|Default|GetCurrentTile)
    (:then
      (Default|ActivateTreasure _currenttile false)
      (bind _treasure (Variables|/Game/Blueprints/Labyrinth/Tile/BP_LabyrinthTile.BP_LabyrinthTile_C|GetTreasure _currenttile)
        (:then
          (EventDispatchers|UnbindallEventsfromOnTreasureGrabbed _treasure))
        (:else)))
    (:else)))

(fn HandleMummyDice
  (LocalVariables|SetAmountSteps (Math|Random|RandomIntegerinRange 0 5))
  (bind _extrasteps (Dice|ResetExplorerDice))
  (LocalVariables|SetAmountExtraSteps _extrasteps)
  (CallFunction|CLIRollDiceMummy (LocalVariables|GetAmountExtraSteps) (LocalVariables|GetAmountSteps)))

(fn OnCaughtbyMummy
  (params (IsExplorer :type Boolean))
  (if IsExplorer
    (Math|Integer|DecrementInt (Variables|Default|GetLives)
      (:%20%20
        (Default|TeleporttoSpawn (Variables|Default|GetControlledPawn))
        (Default|CallOnExplorerCaught (General|GetPlayerName))))
    (else
      (Math|Integer|IncrementInt (Variables|Default|GetLives)
        (:%20%20
          (Turn|UpdateSteps)
          (CallFunction|CLIonUpdateSteps (Variables|Default|GetPlayerSteps))))))
  (CallFunction|CLIonUpdateLives (Variables|Default|GetLives)))

(fn UpdateLives
  (params (Lives :type Integer))
  (bind _output_get (Variables|Default|SetLives Lives))
  (bind _playerhud (Variables|Default|GetPlayerHud)
    (:then
      (Default|UpdateLives _playerhud _output_get))
    (:else)))

(fn InitializeLives
  (if (General|IsExplorer)
    (Variables|Default|SetLives 3)
    (else
      (Variables|Default|SetLives 0))))

(fn UpdateSteps
  (params (Steps :type Integer))
  (bind _output_get (Variables|Default|SetPlayerSteps (Math|Integer|Clamp(Integer) Steps 0 10)))
  (bind _playerhud (Variables|Default|GetPlayerHud)
    (:then
      (Default|UpdateSteps _playerhud _output_get))
    (:else)))

(fn OnRepPlayerSteps
  (bind _playerhud (Variables|Default|GetPlayerHud)
    (:then
      (Default|UpdateSteps _playerhud (Variables|Default|GetPlayerSteps)))
    (:else)))

(fn OnRepLives
  (bind _playerhud (Variables|Default|GetPlayerHud)
    (:then
      (Default|UpdateLives _playerhud (Variables|Default|GetLives)))
    (:else)))

(fn GetPlayerName
  (return "PlayerName"))