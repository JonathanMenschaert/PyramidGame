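; BP_LobbyController is the lobby player controller that shows the game start menu and relays player choices to game logic.
; On BeginPlay, the local controller creates WBP_StartGame, shows the cursor and switches to UI-only input.
; Start-game and player-type requests pass through SER-prefixed events, apparently server RPCs.
; These call StartGame on GM_Lobby and SetPlayerType on the controller's BP_PlayerState.
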(event Custom|OnGameStart
  (CallFunction|SERonGameStart))

(event Custom|SER_ChangePlayerType
  (params (PlayerType :type EPlayerType%20Enum :default "EXPLORER"))
  (bind _asbp_player_state (Utilities|Casting|CastToBP_PlayerState (Variables|GetPlayerState)))
  (Class|PlayerStateLabyrinth|SetPlayerType _asbp_player_state PlayerType))

(event Custom|ChangePlayerType
  (params (PlayerType :type EPlayerType%20Enum :default "EXPLORER"))
  (CallFunction|SERChangePlayerType PlayerType))

(event Custom|SER_OnGameStart
  (bind _asgm_lobby (Utilities|Casting|CastToGM_Lobby (Game|GetGameMode)))
  (Default|StartGame _asgm_lobby))

(event EventBeginPlay
  (if (Pawn|IsLocalController)
    (bind _returnvalue (UserInterface|CreateWidget "/Game/UserInterface/Widgets/Menu/WBP_StartGame.WBP_StartGame_C" self))
    (UserInterface|Viewport|AddtoViewport _returnvalue 0)
    (Variables|Default|SetbShowMouseCursor true)
    (Input|SetInputModeUIOnly self _returnvalue "DoNotLock" false)))

(fn ConstructionScript)