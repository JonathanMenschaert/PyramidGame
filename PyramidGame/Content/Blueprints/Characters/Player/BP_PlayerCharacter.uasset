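; Player character for a networked, turn-based labyrinth game, handling tile entry, punch interactions, dice attachment to the camera and teleporting to spawn.
; Turn start and end swap a replicated collision profile, and overlaps with TileDetector components report valid tiles.
; Map and notebook actions set animation states locally and relay them to remote copies via server-to-multicast events.
; ABP_Character callbacks spawn hand-held UI items and forward open and close events.
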(event OnComponentBeginOverlap(CapsuleComponent)
  (params (OverlappedComponent :type Primitive%20Component%20Object%20Reference) (OtherActor :type Actor%20Object%20Reference) (OtherComp :type Primitive%20Component%20Object%20Reference) (OtherBodyIndex :type Integer) (bFromSweep :type Boolean) (SweepResult :type Hit%20Result%20Structure%20%28by%20ref%29))
  (if (Components|ComponentHasTag OtherComp "TileDetector")
    (bind _asbp_labyrinth_tile (Utilities|Casting|CastToBP_LabyrinthTile OtherActor))
    (if (Default|IsValidTile _asbp_labyrinth_tile)
      (Default|CallOnTileEntered _asbp_labyrinth_tile))))

(event Custom|OnTurnStart
  (Variables|Collision|SetCurrentCollisionProfile (Variables|Collision|GetTurnCollisionProfile)))

(event Custom|OnTurnEnd
  (Variables|Collision|SetCurrentCollisionProfile (Variables|Collision|GetIdleCollisionProfile)))

(event Custom|UpdateCollisionProfile
  (Collision|SetCollisionProfileName (Variables|Default|GetCapsuleComponent) (Variables|Collision|GetCurrentCollisionProfile) true :!class /Script/Engine.PrimitiveComponent))

(event Custom|OnPunch
  (if (not (Pawn|IsLocallyControlled))
    (CallFunction|PunchAnimation)))

(event Custom|PunchAnimation
  (Variables|Animation|SetAnimationState "NewEnumerator4")
  (Variables|Default|SetAllowedToInteract false)
  (Utilities|FlowControl|Delay 0.5)
  (Variables|Default|SetAllowedToInteract true)
  (if (Utilities|Enum|Equal(Enum) (Variables|Animation|GetAnimationState) "NewEnumerator4")
    (Variables|Animation|SetAnimationState "NewEnumerator0")))

(event EventBeginPlay
  (Transformation|AttachComponentToComponent (Variables|Default|GetCameraBoom) (Variables|Character|GetMesh) "Neck" "KeepRelative" "KeepRelative" "SnapToTarget" true)
  (CallFunction|SetupAnimations)
  (Variables|Default|SetSpawnPoint (Transformation|GetActorLocation)))

(event EventOnInteractionFailed
  (params (isServer :type Boolean))
  (CallFunction|HandlePunch isServer))

(event EventOnInteractionSuccess
  (params (isServer :type Boolean))
  (CallFunction|HandlePunch isServer))

(event Custom|OpenMap
  ;[1 1 1] Open Map UI
  (CallFunction|SEROpenMap)
  (Variables|Animation|SetAnimationState "NewEnumerator1"))

(event Custom|SER_OpenMap
  ;[1 1 1] Open Map UI
  (CallFunction|MULOpenMap))

(event Custom|NextPageUIAnimation
  ;[1 1 1] UI Item Controls
  (Default|NextPage (Variables|Animation|GetUIItem)))

(event Custom|SetupAnimations
  ;[1 1 1] Setup Animation bindings
  (bind _asabp_character (Utilities|Casting|CastToABP_Character (Components|SkeletalMesh|GetAnimInstance (Variables|Character|GetMesh))))
  (bind _output_get (Variables|Animation|SetAnimCharacter _asabp_character))
  (Utilities|IsValid _output_get
    (:Is%20Valid
      (EventDispatchers|BindEventtoOnCloseUI (Variables|Animation|GetAnimCharacter) (EventDispatchers|CreateEvent :!event Custom|CloseUIAnimation))
      (EventDispatchers|BindEventtoOnOpenUI (Variables|Animation|GetAnimCharacter) (EventDispatchers|CreateEvent :!event Custom|OpenUIAnimation))
      (EventDispatchers|BindEventtoOnPutAwayItem (Variables|Animation|GetAnimCharacter) (EventDispatchers|CreateEvent :!event DestroyUIItem))
      (EventDispatchers|BindEventtoOnTakeItem (Variables|Animation|GetAnimCharacter) (delegate Custom|OnSpawnUIItem))
      (EventDispatchers|BindEventtoOnFinishClosingUI (Variables|Animation|GetAnimCharacter) (delegate Custom|OnFinishClosingUI))
      (EventDispatchers|BindEventtoOnFinishOpeningUI (Variables|Animation|GetAnimCharacter) (delegate Custom|OnFinishOpeningUI))
      (EventDispatchers|BindEventtoOnStartClosingUI (Variables|Animation|GetAnimCharacter) (delegate Custom|OnStartClosingUI)))))

(event Custom|OnSpawnUIItem
  ;[1 1 1] Setup Animation bindings
  (switch Utilities|FlowControl|Switch|SwitchonE_CharacterState (Variables|Animation|GetAnimationState)
    (:NewEnumerator1
      (CallFunction|SpawnUIItem "/Game/Blueprints/Items/Map/BP_MapItem.BP_MapItem_C"))
    (:NewEnumerator2
      (CallFunction|SpawnUIItem "/Game/Blueprints/Items/Notebook/BP_BookItem.BP_BookItem_C"))))

(event Custom|OpenBook
  ;[1 1 1] Open Notebook UI
  (CallFunction|SEROpenBook)
  (Variables|Animation|SetAnimationState "NewEnumerator2"))

(event Custom|SER_OpenBook
  ;[1 1 1] Open Notebook UI
  (CallFunction|MULOpenBook))

(event Custom|MUL_OpenBook
  ;[1 1 1] Open Notebook UI
  (if (not (Pawn|IsLocallyControlled))
    (Variables|Animation|SetAnimationState "NewEnumerator2")))

(event Custom|OnFinishClosingUI
  ;[1 1 1] Setup Animation bindings
  (Default|CallOnUIClosed))

(event Custom|OnFinishOpeningUI
  ;[1 1 1] Setup Animation bindings
  (Default|CallOnUIOpened))

(event Custom|MUL_OpenMap
  ;[1 1 1] Open Map UI
  (if (not (Pawn|IsLocallyControlled))
    (Variables|Animation|SetAnimationState "NewEnumerator1")))

(event Custom|OnStartClosingUI
  ;[1 1 1] Setup Animation bindings
  (Default|CallOnUIStartClosing))

(event Custom|CloseUI
  ;[1 1 1] Close UI
  (CallFunction|SERCloseUI)
  (Variables|Animation|SetAnimationState "NewEnumerator3"))

(event Custom|SER_CloseUI
  ;[1 1 1] Close UI
  (CallFunction|MULCloseUI))

(event Custom|MUL_CloseUI
  ;[1 1 1] Close UI
  (if (not (Pawn|IsLocallyControlled))
    (Variables|Animation|SetAnimationState "NewEnumerator3")))

(event Custom|OpenUIAnimation
  ;[1 1 1] UI Item Controls
  (Default|OpenUIItem (Variables|Animation|GetUIItem)))

(event Custom|CloseUIAnimation
  ;[1 1 1] UI Item Controls
  (Default|CloseUIItem (Variables|Animation|GetUIItem)))

(event Custom|PreviousPageUIAnimation
  ;[1 1 1] UI Item Controls
  (Default|PreviousPage (Variables|Animation|GetUIItem)))

(fn ConstructionScript)

(fn OnRepCurrentCollisionProfile
  (CallFunction|UpdateCollisionProfile))

(fn EnableInteraction
  (Variables|Default|SetAllowedToInteract true))

(fn CanInteract
  (return (Variables|Default|GetAllowedToInteract)))

(fn GetTraceStartPoint
  (bind _camera (Variables|Default|GetCamera))
  (return (Math|Vector|GetForwardVector (Transformation|GetWorldRotation _camera)) (Transformation|GetWorldLocation _camera)))

(fn SpawnUIItem
  (params (Class :type BP%20Base%20UI%20Item%20Class%20Reference))
  (bind _returnvalue (Game|SpawnActorfromClass Class (Transformation|GetActorTransform) "Undefined" "MultiplyWithRoot" 0 0))
  (bind _output_get (Variables|Animation|SetUIItem _returnvalue))
  (Transformation|AttachComponentToComponent _output_get (Variables|Character|GetMesh) "HandRSocket" "SnapToTarget" "SnapToTarget" "SnapToTarget" true))

(fn DestroyUIItem
  (bind _uiitem (Variables|Animation|GetUIItem)
    (:then
      (Actor|DestroyActor _uiitem)
      (Variables|Animation|SetUIItem 0))
    (:else)))

(fn AddDiceScreen
  (params (DiceHolder :type BP%20Dice%20Holder%20Object%20Reference) (IsExplorer :type Boolean))
  (Default|InitializeDice DiceHolder IsExplorer)
  (Transformation|AttachComponentToComponent DiceHolder (Variables|Default|GetCamera) "None" "SnapToTarget" "SnapToTarget" "KeepRelative" true))

(fn TeleporttoSpawn
  (Transformation|SetActorLocation (Variables|Default|GetSpawnPoint) false true))

(fn HandlePunch
  (params (IsServer :type Boolean))
  (if (Variables|Default|GetAllowedToInteract)
    (if IsServer
      (CallFunction|OnPunch)
      (else
        (CallFunction|PunchAnimation)))))