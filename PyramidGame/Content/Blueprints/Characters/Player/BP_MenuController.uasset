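; Player controller for the main menu that shows the menu widget with UI-only input and a custom widget mouse cursor.
; On BeginPlay, the local controller creates the menu and cursor widgets, adds the UI input mapping context and hides the system cursor.
; Tick moves the cursor widget to the DPI-scaled mouse position every frame, a noted workaround for input not working properly with widgets.
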(event EventBeginPlay
  (if (Pawn|IsLocalController)
    (bind _returnvalue (UserInterface|CreateWidget "/Game/UserInterface/Widgets/Menu/WBP_MainMenu.WBP_MainMenu_C" self))
    (UserInterface|Viewport|AddtoViewport _returnvalue 0)
    (Input|SetInputModeUIOnly self _returnvalue "DoNotLock" true)
    (Input|AddMappingContext (PlayerController|LocalPlayerSubsystems|GetEnhancedInputLocalPlayerSubsystem) "/Game/Blueprints/Characters/Player/Input/IMC_UserInterface.IMC_UserInterface" 0 "(bIgnoreAllPressedKeysUntilRelease=True,bForceImmediately=False,bNotifyUserSettings=False)")
    (bind _returnvalue_2 (UserInterface|CreateWidget "/Game/UserInterface/Widgets/Menu/WBP_MouseCursor.WBP_MouseCursor_C"))
    (bind _output_get (Variables|Default|SetMouseCursor _returnvalue_2))
    (UserInterface|Viewport|AddtoViewport _output_get 0)
    (CallFunction|UpdateMousePosition)
    (Variables|Default|SetbShowMouseCursor false)))

(event EventTick
  (params (DeltaSeconds :type Float%20%28single-precision%29))
  ;[1 1 1] Not a great solution, but the Input System refuses to work properly with the Widgets
  (CallFunction|UpdateMousePosition))

(fn ConstructionScript)

(fn UpdateMousePosition
  (bind _self self)
  (bind (_locationx _locationy) (Class|WidgetLayoutLibrary|GetMousePositionScaledbyDPI _self))
  (bind _mousecursor (Variables|Default|GetMouseCursor)
    (:then
      (Class|UserWidget|SetPositioninViewport _mousecursor (Math|Vector2D|MakeVector2D _locationx _locationy) false))
    (:else)))