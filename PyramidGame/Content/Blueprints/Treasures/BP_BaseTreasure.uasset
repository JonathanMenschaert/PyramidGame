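; Base treasure actor that the player can interact with to grab it, tagged with a zone index and a treasure name.
; Interacting while it is activated prints a debug message, fires OnTreasureGrabbed with zone and name, then destroys the actor.
; SetZoneIndex clamps the zone to byte range and writes it to the mesh's custom depth stencil.
; AllowsInteraction always returns true, and the hover events are empty.
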(event EventBeginPlay)

(event Collision|EventActorBeginOverlap
  (params (OtherActor :type Actor%20Object%20Reference)))

(event EventTick
  (params (DeltaSeconds :type Float%20%28single-precision%29)))

(event EventOnInteract
  (if (Variables|Default|GetActivated)
    (Development|PrintString "Treasure here!" true true "(R=1.000000,G=0.044161,B=0.369304,A=1.000000)")
    (Default|CallOnTreasureGrabbed (Variables|Default|GetZoneIdx) (Variables|Default|GetTreasureName))
    (Actor|DestroyActor)))

(event EventOnHoverExit)

(event EventOnHoverEnter)

(fn ConstructionScript)

(fn SetZoneIndex
  (params (ZoneIndex :type Integer))
  (bind _staticmesh (Variables|Default|GetStaticMesh))
  (Variables|Default|SetZoneIdx (Math|Integer|Clamp(Integer) ZoneIndex 0 255))
  (Rendering|SetRenderCustomDepth _staticmesh true)
  (Rendering|SetCustomDepthStencilValue _staticmesh (Variables|Default|GetZoneIdx)))

(fn AllowsInteraction
  (return true))