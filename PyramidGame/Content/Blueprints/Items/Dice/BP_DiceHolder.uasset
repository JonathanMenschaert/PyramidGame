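; BP_DiceHolder spawns and manages a player's dice: six normal dice for an explorer, otherwise one mummy die, each attached to a holder component.
; Rolling starts and stops die by die through self-re-triggering timers that step an index, giving a staggered effect.
; It also pushes supplied values to the dice, can force-stop all at once, toggles selection, reports the selected die's value and destroys the dice.
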(event Custom|InitializeDice
  (params (IsExplorer :type Boolean))
  (CallFunction|SpawnDice IsExplorer))

(event Custom|DestroyDice
  (params (DestroyedActor :type Actor%20Object%20Reference))
  (for _array_element (Variables|Default|GetDice)
    (Actor|DestroyActor _array_element)))

(fn ConstructionScript)

(fn StartRolling
  (Default|SetStatetoRolling (Utilities|Array|Get(acopy) (Variables|Default|GetDice) (Variables|Default|GetInitIndex)))
  (bind _result (Math|Integer|IncrementInt (Variables|Default|GetInitIndex))
    (:%20%20
      (if (< _result (Utilities|Array|Length (Variables|Default|GetDice)))
        (Utilities|Time|SetTimerbyFunctionName 0 "StartRolling" 0.2)
        (else
          (Variables|Default|SetInitIndex 0))))))

(fn UpdateDice
  (params (DieValues :type Array%20of%20Integers))
  (for (_array_element _array_index) (Variables|Default|GetDice)
    (Default|SetNewValue _array_element (Utilities|Array|Get(acopy) DieValues _array_index))))

(fn StopRolling
  (Default|UpdateDie (Utilities|Array|Get(acopy) (Variables|Default|GetDice) (Variables|Default|GetInitIndex)))
  (bind _result (Math|Integer|IncrementInt (Variables|Default|GetInitIndex))
    (:%20%20
      (if (< _result (Utilities|Array|Length (Variables|Default|GetDice)))
        (Utilities|Time|SetTimerbyFunctionName 0 "StopRolling" 0.2)
        (else
          (Variables|Default|SetInitIndex 0))))))

(fn AllowDiceSelection
  (params (AllowSelection :type Boolean))
  (for _array_element (Variables|Default|GetDice)
    (Default|AllowSelection _array_element AllowSelection)))

(fn FindSelectedDieValue
  (for _array_element (Variables|Default|GetDice)
    (if (Variables|/Game/Blueprints/Items/Dice/BP_NormalDie.BP_NormalDie_C|GetIsSelected _array_element)
      (LocalVariables|SetDieValue (Default|GetValuefromState _array_element))))
  (return (LocalVariables|GetDieValue)))

(fn SpawnDice
  (params (IsExplorer :type Boolean))
  (if IsExplorer
    (Variables|Default|SetDieHolders (Utilities|Array|MakeArray (Variables|Default|GetDieHolder1) (Variables|Default|GetDieHolder2) (Variables|Default|GetDieHolder3) (Variables|Default|GetDieHolder4) (Variables|Default|GetDieHolder5) (Variables|Default|GetDieHolder6)))
    (LocalVariables|SetDieClass "/Game/Blueprints/Items/Dice/BP_NormalDie.BP_NormalDie_C")
    (else
      (Variables|Default|SetDieHolders (Utilities|Array|MakeArray (Variables|Default|GetDieHolder7)))
      (LocalVariables|SetDieClass "/Game/Blueprints/Items/Dice/BP_MummyDie.BP_MummyDie_C")))
  (for _array_element (Variables|Default|GetDieHolders)
    (bind _returnvalue (Game|SpawnActorfromClass (LocalVariables|GetDieClass) (Transformation|GetWorldTransform _array_element) "Undefined" "MultiplyWithRoot" 0 0))
    (Utilities|Array|Add (Variables|Default|GetDice) _returnvalue)
    (Transformation|AttachComponentToComponent _returnvalue _array_element "None" "SnapToTarget" "SnapToTarget" "KeepWorld" true)))

(fn ForceStopRolling
  (params (DIeValues :type Array%20of%20Integers))
  (for (_array_element _array_index) (Variables|Default|GetDice)
    (Utilities|IsValid _array_element
      (:Is%20Valid
        (Default|SetNewValue _array_element (Utilities|Array|Get(acopy) DIeValues _array_index))
        (Default|UpdateDie _array_element)))))