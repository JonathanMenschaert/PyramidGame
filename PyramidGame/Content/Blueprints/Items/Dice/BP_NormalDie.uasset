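; BP_NormalDie is a die item that tracks its roll state and face value and supports hover selection.
; Hovering outlines it via skeletal mesh custom depth and marks it selected, when selection is allowed and it can roll.
; A die on Side1 cannot roll or be selected.
; UpdateDie converts the stored value to a side state, while GetValueFromState maps states back through a differently ordered table.
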(event EventOnHoverEnter
  (bind _skeletalmesh (Variables|Default|GetSkeletalMesh))
  (if (and (CallFunction|CanRoll) (Variables|Default|GetAllow%20Selection))
    (Rendering|SetRenderCustomDepth _skeletalmesh true)
    (Rendering|SetCustomDepthStencilValue _skeletalmesh 0)
    (Variables|Default|SetIsSelected true)))

(event EventOnHoverExit
  (Rendering|SetRenderCustomDepth (Variables|Default|GetSkeletalMesh) false)
  (Variables|Default|SetIsSelected false))

(fn ConstructionScript)

(fn SetStatetoRolling
  (if (CallFunction|CanRoll)
    (Variables|Default|SetDieState "NewEnumerator1")))

(fn CanRoll
  (return (Utilities|Enum|NotEqual(Enum) (Variables|Default|GetDieState) "NewEnumerator2")))

(fn SetNewValue
  (params (DieValue :type Integer))
  (Variables|Default|SetDieValue DieValue))

(fn UpdateDie
  (Variables|Default|SetDieState (Utilities|Select :Index (Variables|Default|GetDieValue) :Option%200 "NewEnumerator2" :Option%201 "NewEnumerator3" :Option%202 "NewEnumerator4" :Option%203 "NewEnumerator5" :Option%204 "NewEnumerator6" :Option%205 "NewEnumerator7")))

(fn AllowSelection
  (params (AllowSelection :type Boolean))
  (if (CallFunction|CanRoll)
    (Variables|Default|SetAllow%20Selection AllowSelection)
    (else
      (Variables|Default|SetAllow%20Selection false))))

(fn GetValuefromState
  (return (Utilities|Select :Index (Variables|Default|GetDieState) :NewEnumerator0 0 :NewEnumerator1 0 :NewEnumerator2 0 :NewEnumerator3 3 :NewEnumerator4 1 :NewEnumerator5 4 :NewEnumerator6 2 :NewEnumerator7 5)))

(fn AllowsInteraction
  (return true))