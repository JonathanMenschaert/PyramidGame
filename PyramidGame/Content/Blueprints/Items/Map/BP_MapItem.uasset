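; BP_MapItem is a map item that shows and hides its Widget as the map is toggled.
; On BeginPlay it runs the parent logic, then binds to the ToggleMap event on the ABP_Map animation instance of its Item mesh.
; When that event fires, it sets Widget visibility from the Open or Close item state, so the animation Blueprint drives when the switch happens.
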(event Custom|OnToggleMap
  (bind _widget (Variables|Default|GetWidget))
  (switch Utilities|FlowControl|Switch|SwitchonE_UIItemState (Variables|Default|GetItemState)
    (:NewEnumerator0
      (Rendering|SetVisibility _widget true false))
    (:NewEnumerator1
      (Rendering|SetVisibility _widget false false))))

(event EventBeginPlay
  (|CallParentFunction)
  (bind _asabp_map (Utilities|Casting|CastToABP_Map (Components|SkeletalMesh|GetAnimInstance (Variables|Default|GetItem))))
  (EventDispatchers|BindEventtoToggleMap _asabp_map (delegate Custom|OnToggleMap)))

(fn ConstructionScript
  (|CallParentFunction))